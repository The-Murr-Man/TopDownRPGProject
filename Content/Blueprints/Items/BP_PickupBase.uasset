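; Base Blueprint for item pickups that animates the actor and plays sounds at the start and end of its life.
; BeginPlay starts sinusoidal movement and rotation and plays a ground impact sound at the actor's location.
; Tick applies the calculated location and rotation without sweeping, though the graph does not compute these values itself.
; Destroyed plays the consume sound on any destruction, with no collection logic in this graph.
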(event EventBeginPlay
  (Class|RPGEffectActor|StartSinusoidalMovement)
  (Class|RPGEffectActor|StartRotation)
  (Audio|PlaySoundatLocation (Variables|Default|GetGroundImpactSound) (Transformation|GetActorLocation) "0, 0, 0" 1.0 1.0 0.0 0 0 0 0))

(event EventDestroyed
  (Audio|PlaySoundatLocation (Variables|Default|GetConsumeSound) (Transformation|GetActorLocation) "0, 0, 0" 1.0 1.0 0.0 0 0 0 0))

(event EventTick
  (params (DeltaSeconds :type Float%20%28single-precision%29))
  (Transformation|SetActorLocation (Variables|Default|GetCalculatedLocation) false false)
  (Transformation|SetActorRotation (Variables|Default|GetCalculatedRotation)))

(fn ConstructionScript)