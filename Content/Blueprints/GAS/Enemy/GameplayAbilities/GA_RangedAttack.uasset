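; Enemy ranged attack gameplay ability that fires a projectile at the avatar's combat target.
; On activation it captures the target's location, turns the avatar toward it and plays a random tagged attack montage.
; A gameplay event matching the montage's tag triggers the socket location lookup and spawns the projectile toward the location captured at activation.
; The graph never calls EndAbility.
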(event Ability|EventActivateAbility
  (bind _returnvalue (Ability|GetAvatarActorfromActorInfo))
  (bind _returnvalue_2 (Class|EnemyInterface|GetCombatTarget(Message) _returnvalue))
  (bind _output_get (Variables|Default|SetTargetLocation (Transformation|GetActorLocation _returnvalue_2)))
  (Class|CombatInterface|UpdateFacingTarget(Message) _returnvalue _output_get)
  (bind _returnvalue_3 (Class|CombatInterface|GetAttackMontages(Message) (Ability|GetAvatarActorfromActorInfo)))
  (bind _output_get_2 (Variables|Default|SetTaggedMontage (Class|RPGDamageGameplayAbility|GetRandomTaggedMontagefromArray _returnvalue_3)))
  (|PlayMontageandWaitProxy "None" (.Montage (Utilities|Struct|BreakTaggedMontage _output_get_2)) 1.0 "None" false 1.0 0.0 false
    (:then
      (Ability|Tasks|WaitGameplayEvent (.MontageTag (Utilities|Struct|BreakTaggedMontage _output_get_2)) 0 true
        (:EventReceived
          (Class|CombatInterface|GetCombatSocketLocation(Message) (Ability|GetAvatarActorfromActorInfo) (.MontageTag (Utilities|Struct|BreakTaggedMontage _output_get_2)))
          (Class|RPGProjectileSpell|SpawnProjectile (Variables|Default|GetTargetLocation)))))))

(event Ability|EventOnEndAbility
  (params (bWasCancelled :type Boolean)))