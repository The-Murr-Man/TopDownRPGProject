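; Passive player ability that turns Attributes gameplay events into changes applied through a gameplay effect on the owner.
; It waits for events under the Attributes tag hierarchy and builds a spec from EventBasedEffectClass for each one received.
; The event magnitude fills the exactly matching SetByCaller tag and every other caller tag is zeroed, so one effect class serves many event tags.
; The spec is then applied to self.
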(event Ability|EventActivateAbility
  (bind _returnvalue (Ability|GetAbilitySystemComponentfromActorInfo))
  (Development|PrintString "Listen For events")
  (bind _payload (Ability|Tasks|WaitGameplayEvent "(TagName=\"Attributes\")" 0 false false)
    (:EventReceived
      (Variables|Default|SetEvent%20Tag (.EventTag (Utilities|Struct|BreakGameplayEventData _payload)))
      (Variables|Default|SetEvent%20Magnitude (.EventMagnitude (Utilities|Struct|BreakGameplayEventData _payload)))
      (Variables|Default|SetOutGoingSpec (GameplayEffects|MakeOutgoingSpec _returnvalue (Variables|Default|GetEventBasedEffectClass) 1.0 (GameplayEffects|MakeEffectContext _returnvalue)))
      (for _array_element (Class|RPGAbilitySystemLibrary|CallerMagnitudeTags (Variables|Default|GetEventBasedEffectClass))
        (if (GameplayTags|MatchesTag _array_element (Variables|Default|GetEvent%20Tag) true)
          (Ability|GameplayEffect|AssignTagSetbyCallerMagnitude (Variables|Default|GetOutGoingSpec) (Variables|Default|GetEvent%20Tag) (Variables|Default|GetEvent%20Magnitude))
          (else
            (Ability|GameplayEffect|AssignTagSetbyCallerMagnitude (Variables|Default|GetOutGoingSpec) _array_element 0.0))))
      (GameplayEffects|ApplyGameplayEffectSpecToSelf (Ability|GetAbilitySystemComponentfromActorInfo) (Variables|Default|GetOutGoingSpec)))))